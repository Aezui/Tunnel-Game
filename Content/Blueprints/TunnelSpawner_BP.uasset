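; TunnelSpawner_BP is a spawner actor that builds a chain of Tunnel_BP segments, starting at the player character's location.
; On BeginPlay it places an initial run of tunnels, each new one at the SpawnLocation of the newest segment.
; Each spawned tunnel receives a reference back to the spawner and is told to spawn its wall.
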(event EventBeginPlay
  (CallFunction|SpawnInitialTunnels))

(event Collision|EventActorBeginOverlap
  (params (OtherActor :type Actor%20Object%20Reference)))

(event EventTick
  (params (DeltaSeconds :type Float%20%28single-precision%29)))

(fn ConstructionScript)

(fn SpawnTunnel
  (params (Location :type Vector))
  (bind _returnvalue (Game|SpawnActorfromClass "/Game/Blueprints/Tunnel_BP.Tunnel_BP_C" (Math|Transform|MakeTransform Location "0, 0, 0" "1.000000,1.000000,1.000000") "Undefined" "MultiplyWithRoot" 0 0))
  (bind _output_get (Variables|Default|SetNewestTunnel _returnvalue))
  (Variables|/Game/Blueprints/Tunnel_BP.Tunnel_BP_C|SetTunnelSpawnerref _output_get self)
  (Default|Spawnwall _output_get))

(fn SpawnTunnelatSpawnPoint
  (CallFunction|SpawnTunnel (Transformation|GetWorldLocation (Variables|/Game/Blueprints/Tunnel_BP.Tunnel_BP_C|GetSpawn%20Location (Variables|Default|GetNewestTunnel)))))

(fn SpawnInitialTunnels
  (for _index (range 0 2)
    (Utilities|IsValid (Variables|Default|GetNewestTunnel)
      (:Is%20Valid
        (CallFunction|SpawnTunnelatSpawnPoint))
      (:Is%20Not%20Valid
        (CallFunction|SpawnTunnel (Transformation|GetActorLocation (Game|GetPlayerCharacter 0)))))))