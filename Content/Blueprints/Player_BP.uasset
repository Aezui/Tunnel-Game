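; Player pawn that flies forward along world X at ForwardSpeed every tick while the mouse steers it sideways and vertically.
; Mouse axes add movement input scaled by MouseSpeed, which is consumed at once and applied as a swept, frame-time-scaled local offset.
; BeginPlay hides the cursor and shows the score widget; the GameOver event restores the cursor, switches to UI-only input, shows the game-over widget and pauses.
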(event Custom|GameOver
  (bind _returnvalue (Game|GetPlayerController 0))
  (Variables|/Script/Engine.PlayerController|SetbShowMouseCursor _returnvalue true)
  (Input|SetInputModeUIOnly _returnvalue 0 "DoNotLock" false)
  (bind _returnvalue_2 (UserInterface|CreateWidget "/Game/UI/GameOver_BP.GameOver_BP_C"))
  (UserInterface|Viewport|AddtoViewport _returnvalue_2 0)
  (Game|SetGamePaused true))

(event Collision|EventActorBeginOverlap
  (params (OtherActor :type Actor%20Object%20Reference)))

(event EventTick
  (params (DeltaSeconds :type Float%20%28single-precision%29))
  (Transformation|AddActorWorldOffset (Math|Vector|MakeVector (* DeltaSeconds (Variables|Default|GetForward_Speed)) 0.0 0.0) true))

(event EventBeginPlay
  (bind _returnvalue (Game|GetPlayerController 0))
  (Variables|/Script/Engine.PlayerController|SetbShowMouseCursor _returnvalue false)
  (Input|SetInputModeGameOnly _returnvalue false)
  (bind _returnvalue_2 (UserInterface|CreateWidget "/Game/UI/Score_BP.Score_BP_C"))
  (UserInterface|Viewport|AddtoViewport _returnvalue_2 0))

(event Input|MouseEvents|MouseY
  (params (AxisValue :type Float%20%28single-precision%29))
  (Pawn|Input|AddMovementInput (Transformation|GetActorUpVector) (* AxisValue (Variables|Default|GetMouse_Speed)) false)
  (bind _returnvalue (Class|Pawn|ConsumeMovementInputVector))
  (Transformation|AddActorLocalOffset (* _returnvalue (Utilities|Time|GetWorldDeltaSeconds)) true false))

(event Input|MouseEvents|MouseX
  (params (AxisValue :type Float%20%28single-precision%29))
  (Pawn|Input|AddMovementInput (Transformation|GetActorRightVector) (* AxisValue (Variables|Default|GetMouse_Speed)) false)
  (bind _returnvalue (Class|Pawn|ConsumeMovementInputVector))
  (Transformation|AddActorLocalOffset (* _returnvalue (Utilities|Time|GetWorldDeltaSeconds)) true false))

(fn ConstructionScript)